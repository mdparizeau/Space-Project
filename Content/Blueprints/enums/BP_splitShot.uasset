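; BP_splitShot is a pickup that grants the interacting player extra projectiles, as a split shot power-up.
; On pickup it runs the parent's logic, then calls AddProjectiles on the player.
; It then spawns a BreakAnimator at its own location and passes it an enum value through BreakMessage.
; BeginPlay and construction only defer to the parent class.
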(event `self.ReceiveBeginPlay`
  (`parent.ReceiveBeginPlay`))

(event `/Game/Blueprints/interfaces/BPI_Pickupable.OnPickedUp`
  (params (interactingPlayer :type "/Game/Blueprints/ship Object Reference"))
  (`parent.OnPickedUp` interactingPlayer)
  (`/Game/Blueprints/ship.addProjectiles` interactingPlayer)
  (bind _returnvalue (`|SpawnActorFromClass` "/Game/Blueprints/FXs/breaks/breakAnimator.breakAnimator_C" (`KismetMathLibrary.MakeTransform` (`self.K2_GetActorLocation`)) "AlwaysSpawn" "MultiplyWithRoot" null null))
  (message `/Game/Blueprints/interfaces/BPI_break.break` _returnvalue "NewEnumerator1"))

(fn `UserConstructionScript`
  (`parent.UserConstructionScript`))