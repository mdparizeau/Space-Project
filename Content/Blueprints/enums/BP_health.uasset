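; BP_health is a health pickup actor built on a parent class that provides the OnPickedUp event.
; It caches BP_gameMode on BeginPlay and calls AddHealth on it when picked up.
; It then spawns a BreakAnimator at its own location and sends it a BreakMessage enum value to trigger the break animation with sound.
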(event `self.ReceiveBeginPlay`
  (`parent.ReceiveBeginPlay`)
  (bind _asbp_game_mode (cast `/Game/Blueprints/BP_gameMode` (`GameplayStatics.GetGameMode`)))
  (set `self.As BP Game Mode` _asbp_game_mode))

(event `/Game/Blueprints/interfaces/BPI_Pickupable.OnPickedUp`
  (params (interactingPlayer :type "/Game/Blueprints/ship Object Reference"))
  ; when "picked up," adds health and spawns break animation which has sound effect
  (`parent.OnPickedUp` interactingPlayer)
  (`/Game/Blueprints/BP_gameMode.addHealth` (`self.As BP Game Mode`))
  (bind _returnvalue (`|SpawnActorFromClass` "/Game/Blueprints/FXs/breaks/breakAnimator.breakAnimator_C" (`KismetMathLibrary.MakeTransform` (`self.K2_GetActorLocation`)) "AlwaysSpawn" "MultiplyWithRoot" null null))
  (message `/Game/Blueprints/interfaces/BPI_break.break` _returnvalue "NewEnumerator2"))

(fn `UserConstructionScript`
  (`parent.UserConstructionScript`))