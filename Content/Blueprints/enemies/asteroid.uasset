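; Asteroid enemy that spins its cube mesh through physics and destroys itself once it passes the left boundary.
; On hit it plays a collision sound, knocks the other component away with partly random velocity, sets Collided, then zeroes that velocity after a delay.
; EndPlay randomly drops shield and health pickups and spawns a break animator, so this also runs on off-screen removal.
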(event `self.ReceiveBeginPlay`
  ; setup, set velocity to start spinning
  (`parent.ReceiveBeginPlay`)
  (`PrimitiveComponent.SetPhysicsAngularVelocityInDegrees` (`self.Cube`) (0.0 0.0 50.0) false "None"))

(event `self.ReceiveTick`
  (params (DeltaSeconds :type "Float (single-precision)"))
  (bind _returnvalue_x (`KismetMathLibrary.BreakVector` (`self.K2_GetActorLocation`)))
  ; if asteroid reaches all the way to the left, destroy actor
  (`/Engine/EditorBlueprintResources/StandardMacros.IsValid` "asteroid"
    (:`Is Valid`
      (if (<= _returnvalue_x -1300.0)
        (`self.K2_DestroyActor`)))))

(event `self.Cube.OnComponentHit`
  (params (HitComponent :type "PrimitiveComponent Object Reference") (OtherActor :type "Actor Object Reference") (OtherComp :type "PrimitiveComponent Object Reference") (NormalImpulse :type "Vector Structure") (Hit :type "HitResult Structure (by ref)"))
  (bind _movespeed (`self.moveSpeed`))
  ; collide w/ something, push it, then reset its velocity
  (`GameplayStatics.SpawnSoundAtLocation` "/Game/SFX/collision.collision" NormalImpulse (struct) 1.0 1.0 0.0 null null)
  (`PrimitiveComponent.SetPhysicsLinearVelocity` OtherComp (`KismetMathLibrary.MakeVector` (* _movespeed -1.5) (* _movespeed (`KismetMathLibrary.RandomFloatInRange` -1.0 1.0))) false "None")
  (`/Engine/EditorBlueprintResources/StandardMacros.IsValid` HitComponent
    (:`Is Valid`
      (set `self.collided` true)
      (`KismetSystemLibrary.Delay` 2.0))
    (:`Is Not Valid`
      _))
  (`PrimitiveComponent.SetPhysicsLinearVelocity` OtherComp (0.0 0.0 0.0) false "None"))

(event `self.ReceiveEndPlay`
  (params (EndPlayReason :type "EEndPlayReason Enum" :default "Destroyed"))
  (bind _returnvalue (`self.K2_GetActorLocation`))
  ; on death
  ;; 30% chance to spawn shield
  (if (== (`KismetMathLibrary.RandomIntegerInRange` 0 2) 2)
    (`|SpawnActorFromClass` "/Game/Blueprints/enums/BP_shield.BP_shield_C" (`KismetMathLibrary.MakeTransform` (`self.K2_GetActorLocation`)) "Undefined" "MultiplyWithRoot" null null))
  ;; 10% chance to spawn health
  (if (== (`KismetMathLibrary.RandomIntegerInRange` 0 9) 9)
    (`|SpawnActorFromClass` "/Game/Blueprints/enums/BP_health.BP_health_C" (`KismetMathLibrary.MakeTransform` _returnvalue) "Undefined" "MultiplyWithRoot" null null))
  (bind _returnvalue_2 (`|SpawnActorFromClass` "/Game/Blueprints/FXs/breaks/breakAnimator.breakAnimator_C" (`KismetMathLibrary.MakeTransform` _returnvalue) "AlwaysSpawn" "MultiplyWithRoot" null null))
  (message `/Game/Blueprints/interfaces/BPI_break.break` _returnvalue_2 "NewEnumerator0"))

(fn `UserConstructionScript`
  (`parent.UserConstructionScript`))