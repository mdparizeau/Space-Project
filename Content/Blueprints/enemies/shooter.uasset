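; Shooter enemy that targets the player pawn, fires a BlueProj from its FirePoint every second with sound, and damages player health on overlap.
; Tick turns it toward the player via an interpolated look-at without setting location, and destroys it past a left X limit.
; EndPlay, which also runs on that off-limit destroy, randomly drops split-shot or health pickups and spawns a BreakAnimator.
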(event `self.ReceiveBeginPlay`
  ; set it UP
  (`KismetSystemLibrary.Delay` 0.1)
  (`parent.ReceiveBeginPlay`)
  (set `self.target` (`GameplayStatics.GetPlayerPawn` 0))
  (`self.shoot`))

(event `self.ReceiveActorBeginOverlap`
  (params (OtherActor :type "Actor Object Reference"))
  (bind _as_bp_game_mode (`self.As BP Game Mode`))
  (bind _playerhealth (`/Game/Blueprints/BP_gameMode.playerHealth` _as_bp_game_mode))
  ; damage enemy on overlap
  (if (== OtherActor (`self.target`))
    (set `/Game/Blueprints/BP_gameMode.playerHealth` (`KismetMathLibrary.Clamp` (- _playerhealth 10) 0 100) _as_bp_game_mode)
    (`KismetSystemLibrary.PrintString` (`KismetStringLibrary.Concat_StrStr` "current playerHealth: " (`KismetStringLibrary.Conv_IntToString` _playerhealth)))))

(event `self.ReceiveTick`
  (params (DeltaSeconds :type "Float (single-precision)"))
  (bind (_returnvalue_x _returnvalue_y _returnvalue_z) (`KismetMathLibrary.BreakVector` (`self.K2_GetActorLocation`)))
  (bind _returnvalue (`self.K2_GetActorLocation` (`self.target`)))
  ; same as asteroid: move to left, then destroy
  (`/Engine/EditorBlueprintResources/StandardMacros.IsValid` self
    (:`Is Valid`
      (`/Engine/EditorBlueprintResources/StandardMacros.IsValid` (`self.target`)
        (:`Is Valid`
          (if (<= _returnvalue_x -1300.0)
            (`self.K2_DestroyActor`)
            (else
              (`self.K2_SetActorRotation` (`KismetMathLibrary.FindLookAtRotation` (`KismetMathLibrary.VInterpTo_Constant` (`KismetMathLibrary.MakeVector` _returnvalue_x _returnvalue_y _returnvalue_z) _returnvalue DeltaSeconds (`self.moveSpeed`)) _returnvalue)))))))))

(event `shoot`
  (bind _firepoint (`self.firePoint`))
  ; shooting loop
  (`KismetSystemLibrary.Delay` 1.0 :!label _label)
  (`|SpawnActorFromClass` "/Game/Blueprints/projectiles/blueProj.blueProj_C" (`KismetMathLibrary.MakeTransform` (`SceneComponent.K2_GetComponentLocation` _firepoint) (`SceneComponent.K2_GetComponentRotation` _firepoint)) "Undefined" "MultiplyWithRoot" null null)
  (`GameplayStatics.SpawnSoundAttached` "/Game/SFX/enemyShooting.enemyShooting" (`self.firePoint`) "None" (0.0 0.0 0.0) (struct) "KeepRelativeOffset" false 1.0 1.0 0.0 null null)
  (goto _label))

(event `self.ReceiveEndPlay`
  (params (EndPlayReason :type "EEndPlayReason Enum" :default "Destroyed"))
  (bind _returnvalue (`self.K2_GetActorLocation`))
  ; on death
  ;; 20% chance to spawn splitShot
  (if (== (`KismetMathLibrary.RandomIntegerInRange` 0 4) 4)
    (`|SpawnActorFromClass` "/Game/Blueprints/enums/BP_splitShot.BP_splitShot_C" (`KismetMathLibrary.MakeTransform` (`self.K2_GetActorLocation`)) "Undefined" "MultiplyWithRoot" null null))
  ;; 10% chance to spawn health
  (if (== (`KismetMathLibrary.RandomIntegerInRange` 0 9) 9)
    (`|SpawnActorFromClass` "/Game/Blueprints/enums/BP_health.BP_health_C" (`KismetMathLibrary.MakeTransform` _returnvalue) "Undefined" "MultiplyWithRoot" null null))
  (bind _returnvalue_2 (`|SpawnActorFromClass` "/Game/Blueprints/FXs/breaks/breakAnimator.breakAnimator_C" (`KismetMathLibrary.MakeTransform` _returnvalue (struct) (1.2 1.0 0.6)) "AlwaysSpawn" "MultiplyWithRoot" null null))
  (message `/Game/Blueprints/interfaces/BPI_break.break` _returnvalue_2 "NewEnumerator0"))

(fn `UserConstructionScript`
  (`parent.UserConstructionScript`))