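; Suicide bomber enemy that homes in on the player and costs them health on contact.
; Each tick it moves horizontally toward the player while facing them, with speed set to the remaining 2D distance, so it slows as it closes in.
; Any overlap destroys it and decrements the game mode's enemy count.
; EndPlay adds score, spawns an explosion and sometimes drops health; the power-shot drop is unconnected.
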(event `self.ReceiveBeginPlay`
  ; gets reference to player, sets baseDeathTime
  (set `self.target` (`GameplayStatics.GetPlayerPawn` 0))
  (bind _asbp_game_mode (cast `/Game/Blueprints/BP_gameMode` (`GameplayStatics.GetGameMode`)))
  (set `self.As BP Game Mode_0` _asbp_game_mode))

(event `self.ReceiveTick`
  (params (DeltaSeconds :type "Float (single-precision)"))
  (bind (_returnvalue_x _returnvalue_y _returnvalue_z) (`KismetMathLibrary.BreakVector` (`self.K2_GetActorLocation`)))
  (bind (_returnvalue_x_2 _returnvalue_y_2) (`KismetMathLibrary.BreakVector` (`self.K2_GetActorLocation`)))
  (bind _returnvalue (`self.K2_GetActorLocation` (`self.target`)))
  (bind (_returnvalue_x_3 _returnvalue_y_3) (`KismetMathLibrary.BreakVector` (`self.K2_GetActorLocation` (`self.target`))))
  (bind _returnvalue_2 (`KismetMathLibrary.VInterpTo_Constant` (`self.K2_GetActorLocation`) _returnvalue DeltaSeconds (`self.moveSpeed`)))
  (bind (_returnvalue_roll _returnvalue_pitch _returnvalue_yaw) (`KismetMathLibrary.BreakRotator` (`KismetMathLibrary.FindLookAtRotation` _returnvalue_2 _returnvalue)))
  ; move and rotate toward target every frame
  (`self.K2_SetActorLocationAndRotation` (`KismetMathLibrary.MakeVector` (.x _returnvalue_2) (.y _returnvalue_2) _returnvalue_z) (`KismetMathLibrary.MakeRotator` 0.0 0.0 _returnvalue_yaw))
  ; get distance between enemy and target
  (set `self.moveSpeed` (`KismetMathLibrary.Distance2D` (`KismetMathLibrary.MakeVector2D` _returnvalue_x_2 _returnvalue_y_2) (`KismetMathLibrary.MakeVector2D` _returnvalue_x_3 _returnvalue_y_3))))

(event `self.ReceiveActorBeginOverlap`
  (params (OtherActor :type "Actor Object Reference"))
  (bind _as_bp_game_mode_0 (`self.As BP Game Mode_0`))
  (bind _playerhealth (`/Game/Blueprints/BP_gameMode.playerHealth` _as_bp_game_mode_0))
  ; spawns explosion after death
  (if (== OtherActor (`self.target`))
    (set `/Game/Blueprints/BP_gameMode.playerHealth` (`KismetMathLibrary.Clamp` (- _playerhealth 10) 0 100) _as_bp_game_mode_0)
    (`KismetSystemLibrary.PrintString` (`KismetStringLibrary.Concat_StrStr` "current playerHealth: " (`KismetStringLibrary.Conv_IntToString` _playerhealth))))
  (`self.K2_DestroyActor`)
  (bind _result (`/Engine/EditorBlueprintResources/StandardMacros.DecrementInt` (`/Game/Blueprints/BP_gameMode.enemiesToDefeat` _as_bp_game_mode_0))
    (:`  `
      (`KismetSystemLibrary.PrintString` (`KismetStringLibrary.Conv_IntToString` _result)))))

(event `self.ReceiveEndPlay`
  (params (EndPlayReason :type "EEndPlayReason Enum" :default "Destroyed"))
  (bind _as_bp_game_mode_0 (`self.As BP Game Mode_0`))
  ; on death
  (set `/Game/Blueprints/BP_gameMode.score` (+ (`/Game/Blueprints/BP_gameMode.score` _as_bp_game_mode_0) 100) _as_bp_game_mode_0)
  (`|SpawnActorFromClass` "/Game/Blueprints/FXs/explosion.explosion_C" (`KismetMathLibrary.MakeTransform` (`self.K2_GetActorLocation`) (struct) (2.0 2.0 2.0)) "Undefined" "MultiplyWithRoot" null null)
  ;; 10% chance to spawn health
  (if (== (`KismetMathLibrary.RandomIntegerInRange` 0 9) 9)
    (`|SpawnActorFromClass` "/Game/Blueprints/enums/BP_health.BP_health_C" (`KismetMathLibrary.MakeTransform` (`self.K2_GetActorLocation`)) "Undefined" "MultiplyWithRoot" null null)))

(fn `UserConstructionScript`
  (`parent.UserConstructionScript`))