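; Game mode for a level-based enemy survival game, handling player health, one-hit shield, score, level progression and game over.
; Tick checks health and remaining enemies; each level-up clears enemies, awards score, shortens base death time and unlocks asteroids, then shooters.
; Looping delay-based spawners place enemies between two spawn points, speeding up when the last spawn dies quickly.
; An extra rush loop spawns more bombers as the level nears its end.
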(event `gameOver`
  ; display gameOver sceen
  (`GameplayStatics.SetGamePaused` true)
  (bind _returnvalue (`GameplayStatics.GetActorOfClass` "/Game/Blueprints/UI/BP_UI_Manager.BP_UI_Manager_C"))
  (bind _output_get (set `/Game/Blueprints/UI/BP_UI_Manager.Widget` "/Game/Blueprints/UI/WBP_GameOver.WBP_GameOver_C" _returnvalue))
  (bind _returnvalue_2 (`|CreateWidget` _output_get))
  (`UserWidget.AddToViewport` _returnvalue_2 0))

(event `self.ReceiveBeginPlay`
  ; set enemies' BDTs and start enemy spawning
  (`KismetSystemLibrary.Delay` 0.2)
  (bind _outactors (`GameplayStatics.GetAllActorsOfClass` "/Game/Blueprints/BP_spawnLocation.BP_spawnLocation_C"))
  (set `self.spawnLocations` _outactors)
  (`self.setCustomBDTs`)
  (`self.spawnEnemies`)
  (`KismetSystemLibrary.PrintString` (`KismetStringLibrary.Concat_StrStr` "initial playerHealth: " (`KismetStringLibrary.Conv_IntToString` (`self.playerHealth`))))
  (set `self.score` 0))

(event `self.ReceiveTick`
  (params (DeltaSeconds :type "Float (single-precision)"))
  (bind _playerhealth (`self.playerHealth`))
  (bind _instancehealth (`self.instanceHealth`))
  ; check if game's over
  (if (<= (`self.playerHealth`) 0)
    (`self.gameOver`)
    (else
      ; did the player get the shield pickup?
      (if (`self.shieldActivated`)
        (set `self.instanceHealth` (`self.playerHealth`))
        (set `self.shieldActivated` false)
        (set `self.isShieldActive` true)
        (else
          ; does the player have the shield pickup?
          (if (`self.isShieldActive`)
            ; does the player need to use the shield pickup?
            (if (>= _playerhealth _instancehealth)
              (set `self.instanceHealth` _playerhealth)
              (else
                (set `self.playerHealth` _instancehealth)
                (set `self.isShieldActive` false))))))
      ; If player defeats enough enemies, level is ended
      (if (<= (`self.enemiesToDefeat`) 0)
        (`self.increment level`)
        ; prints vaiable values for debugging
        (`KismetSystemLibrary.PrintString` (`KismetStringLibrary.Concat_StrStr` "Level: " (`KismetStringLibrary.Conv_IntToString` (`self.level`))))
        (`KismetSystemLibrary.PrintString` (`KismetStringLibrary.Concat_StrStr` "Player Score: " (`KismetStringLibrary.Conv_IntToString` (`self.score`))))
        (`KismetSystemLibrary.PrintString` (`KismetStringLibrary.Concat_StrStr` "B_BDT: " (`KismetStringLibrary.Conv_DoubleToString` (`self.bomberBDT`))))))))

(event `increment level`
  (bind _level (`self.level`))
  ; when level completed, destroys all enemies, increases player score, increments level, and adjusts new enemiesToDefeat and baseDeathTime variables
  (for _array_element (`self.enemiesAlive`)
    (`/Engine/EditorBlueprintResources/StandardMacros.IsValid` _array_element
      (:`Is Valid`
        (`self.K2_DestroyActor` _array_element))))
  (set `self.score` (+ (`self.score`) (* (`self.level`) 500)))
  (bind _result (`/Engine/EditorBlueprintResources/StandardMacros.IncrementInt` _level)
    (:`  `
      (set `self.enemiesToDefeat` (+ (* _result _level) 10))
      (set `self.baseDeathTime` (* (`self.baseDeathTime`) 0.8))
      ;; start spawning certain enemies at certain levels
      (`self.setCustomBDTs`)
      (if (== (`self.level`) 2)
        (`self.spawnAsteroids`)
        (elif (== (`self.level`) 3)
          (`self.spawnShooters`))))))

(event `addHealth`
  (bind _playerhealth (`self.playerHealth`))
  ; add health for health pickup
  (set `self.playerHealth` (`KismetMathLibrary.Clamp` (+ _playerhealth 20) 0 100))
  (`KismetSystemLibrary.PrintString` (`KismetStringLibrary.Concat_StrStr` "HEALTH ADDED!" (`KismetStringLibrary.Conv_IntToString` _playerhealth))))

(event `spawnEnemies`
  ; organizes initial enemy spawners
  (`self.EOL_Rush`)
  (`self.spawnBombers`))

(event `setCustomBDTs`
  (bind _basedeathtime (`self.baseDeathTime`))
  ; organizes all BDT setters
  (set `self.bomberBDT` (* _basedeathtime 0.8))
  (set `self.asteroidBDT` (* _basedeathtime 0.5))
  (set `self.shooterBDT` (* _basedeathtime 0.9))
  (set `self.rushBDT` (* _basedeathtime 0.5)))

(event `spawnBombers`
  (bind _bomberbdt (`self.bomberBDT`))
  (bind _returnvalue (`KismetMathLibrary.RandomFloatInRange` (* _bomberbdt 0.8) (* _bomberbdt 1.2)))
  ; spawns bombers w/in a range of time
  ; PRINT STATEMENTS FOR DEBUGGING
  (`KismetSystemLibrary.PrintString` (`KismetStringLibrary.Conv_DoubleToString` (`self.bomberBDT`)))
  (if (`self.gameIsOngoing`) :!label _label
    (bind _returnvalue_2 (`|SpawnActorFromClass` "/Game/Blueprints/enemies/suicideBomber.suicideBomber_C" (`KismetMathLibrary.MakeTransform` (`self.determineSpawnLocationNEW`)) "Undefined" "MultiplyWithRoot" null null))
    (`KismetArrayLibrary.Array_Add` (`self.enemiesAlive`) _returnvalue_2)
    (`KismetSystemLibrary.PrintString` "ENEMY SPAWNED")
    (`KismetSystemLibrary.Delay` (/ _returnvalue 2.0))
    (`KismetSystemLibrary.PrintString` (`KismetStringLibrary.Concat_StrStr` "DELAY 1 COMPLETE" "B_BDT: " (`KismetStringLibrary.Conv_DoubleToString` (`self.bomberBDT`))))
    (if (`KismetSystemLibrary.IsValid` _returnvalue_2)
      (`KismetSystemLibrary.Delay` _returnvalue)
      (`KismetSystemLibrary.PrintString` (`KismetStringLibrary.Concat_StrStr` "DELAY 2 COMPLETE" "B_BDT: " (`KismetStringLibrary.Conv_DoubleToString` (`self.bomberBDT`))))
      (if (`KismetSystemLibrary.IsValid` _returnvalue_2)
        (goto _label)
        (else
          (set `self.bomberBDT` (* (`self.bomberBDT`) 0.875))
          (goto _label)))
      (else
        (set `self.bomberBDT` (* (`self.bomberBDT`) 0.75))
        (goto _label)))))

(event `spawnAsteroids`
  (bind _asteroidbdt (`self.asteroidBDT`))
  (bind _returnvalue (`KismetMathLibrary.RandomFloatInRange` (* _asteroidbdt 0.8) (* _asteroidbdt 1.2)))
  ; spawns asteroids w/in a range of time
  ; PRINT STATEMENTS FOR DEBUGGING
  (`KismetSystemLibrary.PrintString` (`KismetStringLibrary.Conv_DoubleToString` (`self.asteroidBDT`)))
  (if (`self.gameIsOngoing`) :!label _label_2
    (bind _returnvalue_2 (`|SpawnActorFromClass` "/Game/Blueprints/enemies/asteroid.asteroid_C" (`KismetMathLibrary.MakeTransform` (`self.determineSpawnLocationNEW`)) "Undefined" "MultiplyWithRoot" null null))
    (`KismetArrayLibrary.Array_Add` (`self.enemiesAlive`) _returnvalue_2)
    (`KismetSystemLibrary.PrintString` "ENEMY SPAWNED")
    (`KismetSystemLibrary.Delay` (/ _returnvalue 2.0))
    (`KismetSystemLibrary.PrintString` (`KismetStringLibrary.Concat_StrStr` "DELAY 1 COMPLETE" "A_BDT: " (`KismetStringLibrary.Conv_DoubleToString` (`self.asteroidBDT`))))
    (if (`KismetSystemLibrary.IsValid` _returnvalue_2)
      (`KismetSystemLibrary.Delay` _returnvalue)
      (`KismetSystemLibrary.PrintString` (`KismetStringLibrary.Concat_StrStr` "DELAY 2 COMPLETE" "A_BDT: " (`KismetStringLibrary.Conv_DoubleToString` (`self.asteroidBDT`))))
      (if (`KismetSystemLibrary.IsValid` _returnvalue_2)
        (goto _label_2)
        (else
          (set `self.asteroidBDT` (* (`self.asteroidBDT`) 0.875))
          (goto _label_2)))
      (else
        (set `self.asteroidBDT` (* (`self.asteroidBDT`) 0.75))
        (goto _label_2)))))

(event `spawnShooters`
  (bind _shooterbdt (`self.shooterBDT`))
  (bind _returnvalue (`KismetMathLibrary.RandomFloatInRange` (* _shooterbdt 0.8) (* _shooterbdt 1.2)))
  ; spawns asteroids w/in a range of time
  ; PRINT STATEMENTS FOR DEBUGGING
  (`KismetSystemLibrary.PrintString` (`KismetStringLibrary.Conv_DoubleToString` (`self.shooterBDT`)))
  (if (`self.gameIsOngoing`) :!label _label_3
    (bind _returnvalue_2 (`|SpawnActorFromClass` "/Game/Blueprints/enemies/shooter.shooter_C" (`KismetMathLibrary.MakeTransform` (`self.determineSpawnLocationNEW`)) "Undefined" "MultiplyWithRoot" null null))
    (`KismetArrayLibrary.Array_Add` (`self.enemiesAlive`) _returnvalue_2)
    (`KismetSystemLibrary.PrintString` "ENEMY SPAWNED")
    (`KismetSystemLibrary.Delay` (/ _returnvalue 2.0))
    (`KismetSystemLibrary.PrintString` (`KismetStringLibrary.Concat_StrStr` "DELAY 1 COMPLETE" "S_BDT: " (`KismetStringLibrary.Conv_DoubleToString` (`self.shooterBDT`))))
    (if (`KismetSystemLibrary.IsValid` _returnvalue_2)
      (`KismetSystemLibrary.Delay` _returnvalue)
      (`KismetSystemLibrary.PrintString` (`KismetStringLibrary.Concat_StrStr` "DELAY 2 COMPLETE" "S_BDT: " (`KismetStringLibrary.Conv_DoubleToString` (`self.shooterBDT`))))
      (if (`KismetSystemLibrary.IsValid` _returnvalue_2)
        (goto _label_3)
        (else
          (set `self.shooterBDT` (* (`self.shooterBDT`) 0.875))
          (goto _label_3)))
      (else
        (set `self.shooterBDT` (* (`self.shooterBDT`) 0.75))
        (goto _label_3)))))

(event `EOL_Rush`
  (bind _spawnlocation (`self.determineSpawnLocationNEW`))
  (bind _level (`self.level`))
  (bind _enemiestodefeat (`self.enemiesToDefeat`))
  (bind _rushbdt (`self.rushBDT`))
  (bind _returnvalue (* (/ (+ (* _level _level) 10) 3) 2))
  ; spawns random amounts of random enemies, increasingly toward the end of the level
  ;; calculates how many enemies should be spawned
  (if (`self.gameIsOngoing`) :!label _label_4
    (`KismetSystemLibrary.Delay` (`KismetMathLibrary.RandomFloatInRange` (* _rushbdt 0.8) (* _rushbdt 1.2)))
    (if (> _enemiestodefeat _returnvalue)
      (set `self.Selection` 0)
      (elif (> _enemiestodefeat (/ _returnvalue 2))
        (set `self.Selection` 1)
        (else
          (set `self.Selection` 2))))
    (for _ (range (+ (`self.Selection`) 1))
      ;; determines which enemy(s) to spawn
      (switch `int` (`KismetMathLibrary.RandomIntegerInRange` 0 2)
        (:`0`
          (bind _returnvalue_2 (`|SpawnActorFromClass` "/Game/Blueprints/enemies/suicideBomber.suicideBomber_C" (`KismetMathLibrary.MakeTransform` _spawnlocation) "Undefined" "MultiplyWithRoot" null null))
          ; adds enemies to array
          (`KismetArrayLibrary.Array_Add` (`self.enemiesAlive`) _returnvalue_2))
        (:`1`
          ;;; change class
          (bind _returnvalue_3 (`|SpawnActorFromClass` "/Game/Blueprints/enemies/suicideBomber.suicideBomber_C" (`KismetMathLibrary.MakeTransform` _spawnlocation) "Undefined" "MultiplyWithRoot" null null))
          (`KismetArrayLibrary.Array_Add` (`self.enemiesAlive`) _returnvalue_3))
        (:`2`
          ;;; change class
          (bind _returnvalue_4 (`|SpawnActorFromClass` "/Game/Blueprints/enemies/suicideBomber.suicideBomber_C" (`KismetMathLibrary.MakeTransform` _spawnlocation) "Undefined" "MultiplyWithRoot" null null))
          (`KismetArrayLibrary.Array_Add` (`self.enemiesAlive`) _returnvalue_4))))
    (goto _label_4)))

(fn `determineSpawnLocationNEW`
  (returns (spawnLocation :type "Vector Structure"))
  (bind (_returnvalue_x _returnvalue_y) (`KismetMathLibrary.BreakVector` (`SceneComponent.K2_GetComponentLocation` (`Actor.RootComponent` (`|GetArrayItem` (`self.spawnLocations`) 1)))))
  (bind (_returnvalue_x_2 _returnvalue_y_2) (`KismetMathLibrary.BreakVector` (`SceneComponent.K2_GetComponentLocation` (`Actor.RootComponent` (`|GetArrayItem` (`self.spawnLocations`))))))
  (return (`KismetMathLibrary.MakeVector` _returnvalue_x_2 (`KismetMathLibrary.Lerp` _returnvalue_y_2 _returnvalue_y (`KismetMathLibrary.RandomFloatInRange` 0.0 1.0)))))

(fn `UserConstructionScript`)