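; Bomb projectile actor that travels a fixed distance along world +X from its spawn point, then explodes.
; Tick moves it with VInterpToConstant, resetting the speed to the remaining 2D distance each frame so it decelerates toward the target.
; Just short of the target it destroys itself and spawns an enlarged Explosion at its location, with no sweep or active overlap handling along the way.
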(event `self.ReceiveBeginPlay`
  (set `self.Target X` (+ (.x (`self.K2_GetActorLocation`)) 750.0)))

(event `self.ReceiveTick`
  (params (DeltaSeconds :type "Float (single-precision)"))
  (bind _returnvalue (`self.K2_GetActorLocation`))
  (bind (_returnvalue_x _returnvalue_y) (`KismetMathLibrary.BreakVector` (`self.K2_GetActorLocation`)))
  (bind _returnvalue_x_2 (`KismetMathLibrary.BreakVector` (`self.K2_GetActorLocation`)))
  (`self.K2_SetActorLocation` (`KismetMathLibrary.VInterpTo_Constant` _returnvalue (`KismetMathLibrary.MakeVector` (`self.Target X`) (.y _returnvalue) (.z _returnvalue)) DeltaSeconds (`self.moveSpeed`)))
  ; get distance between proj and target
  (set `self.moveSpeed` (`KismetMathLibrary.Distance2D` (`KismetMathLibrary.MakeVector2D` _returnvalue_x _returnvalue_y) (`KismetMathLibrary.MakeVector2D` (`self.Target X`) _returnvalue_y)))
  (if (>= _returnvalue_x_2 (- (`self.Target X`) 75.0))
    (`self.K2_DestroyActor`)
    (`|SpawnActorFromClass` "/Game/Blueprints/FXs/explosion.explosion_C" (`KismetMathLibrary.MakeTransform` (`self.K2_GetActorLocation`) (struct) (1.5 1.5 1.5)) "Undefined" "MultiplyWithRoot" null null)))

(fn `UserConstructionScript`
  (`parent.UserConstructionScript`))