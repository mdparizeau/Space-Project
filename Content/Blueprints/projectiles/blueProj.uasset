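; Blue projectile actor that damages the player on contact.
; On BeginPlay it caches the player pawn as its target and a reference to BP_gameMode, which holds the player's health.
; An overlap with the player subtracts a fixed amount from that health, clamped to its valid range, and prints the result.
; The projectile destroys itself on any actor overlap, whether or not it hit the player.
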(event `self.ReceiveBeginPlay`
  ; set it UP
  (set `self.target` (`GameplayStatics.GetPlayerPawn` 0))
  (bind _asbp_game_mode (cast `/Game/Blueprints/BP_gameMode` (`GameplayStatics.GetGameMode`)))
  (set `self.As BP Game Mode` _asbp_game_mode))

(event `self.ReceiveActorBeginOverlap`
  (params (OtherActor :type "Actor Object Reference"))
  (bind _as_bp_game_mode (`self.As BP Game Mode`))
  (bind _playerhealth (`/Game/Blueprints/BP_gameMode.playerHealth` _as_bp_game_mode))
  ; if hit player, dmg
  (if (== OtherActor (`self.target`))
    (set `/Game/Blueprints/BP_gameMode.playerHealth` (`KismetMathLibrary.Clamp` (- _playerhealth 10) 0 100) _as_bp_game_mode)
    (`KismetSystemLibrary.PrintString` (`KismetStringLibrary.Concat_StrStr` "current playerHealth: " (`KismetStringLibrary.Conv_IntToString` _playerhealth))))
  (`self.K2_DestroyActor`))

(fn `UserConstructionScript`
  (`parent.UserConstructionScript`))